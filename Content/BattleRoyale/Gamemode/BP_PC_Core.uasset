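; BP_PC_Core is a player controller in the Battle Royale game mode that handles the in-game menu toggle.
; On BeginPlay it sets game-only input mode.
; The IA_ToggleGameMenu input action creates WG_GameMenu and adds it to the viewport on first use, then reuses that cached widget by switching it between Visible and Collapsed.
; Toggling the menu leaves the input mode unchanged.
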(event `self.ReceiveBeginPlay`
  (`WidgetBlueprintLibrary.SetInputMode_GameOnly` self))

(event `EnhancedInput|/Game/ThirdPerson/Input/Actions/IA_ToggleGameMenu`
  (params (ActionValue :type Boolean) (ElapsedSeconds :type "Float (double-precision)") (TriggeredSeconds :type "Float (double-precision)") (InputAction :type "InputAction Object Reference" :default "/Game/ThirdPerson/Input/Actions/IA_ToggleGameMenu.IA_ToggleGameMenu"))
  (bind _wg_gamemenu (`self.WG_GameMenu`))
  (:`Triggered`
    (`self.WG_GameMenu`
      (:`then`
        (if (`Widget.IsVisible` _wg_gamemenu)
          (`Widget.SetVisibility` _wg_gamemenu "Collapsed")
          (else
            (`Widget.SetVisibility` _wg_gamemenu "Visible"))))
      (:`else`
        (bind _returnvalue (`|CreateWidget` "/Game/BattleRoyale/WIdget/GameWidget/WG_GameMenu.WG_GameMenu_C" self))
        (bind _output_get (set `self.WG_GameMenu` _returnvalue))
        (`UserWidget.AddToViewport` _output_get 0)))))

(fn `UserConstructionScript`)