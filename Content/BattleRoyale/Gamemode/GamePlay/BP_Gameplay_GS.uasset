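; Battle royale game state that runs the pre-match countdown once enough players have connected.
; Player connection notifications update the player count and, at the minimum, set the replicated countdown to 15 once.
; Its OnRep refreshes every countdown widget and calls a one-second delayed decrement, which retriggers the OnRep until zero.
; Nothing here acts on reaching zero, and CheckIfReadyToStart is empty.
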(event `CheckIfReadyToStart`)

(event `/Game/BattleRoyale/Gamemode/Interface/BPI_GameState.Notify_PlayerConnection`
  (bind _returnvalue (`GameplayStatics.GetNumPlayerStates`))
  (set `self.CurrentAmountOfPlayers` _returnvalue)
  (if (>= _returnvalue (`self.MinimumRequiredPlayers`))
    (`/Engine/EditorBlueprintResources/StandardMacros.DoOnce` false
      (:`Completed`
        (set `self.MatchStart_Countdown` 15)))))

(event `Match_Countdown`
  (`KismetSystemLibrary.Delay` 1.0)
  (set `self.MatchStart_Countdown` (- (`self.MatchStart_Countdown`) 1)))

(fn `OnRep_MatchStart_Countdown`
  (bind _matchstart_countdown (`self.MatchStart_Countdown`))
  (`self.Update_MatchCountdownWidget`)
  (if (== _matchstart_countdown 15)
    (`self.Match_Countdown`)
    (elif (not (== _matchstart_countdown 0))
      (`self.Match_Countdown`))))

(fn `Update_MatchCountdownWidget`
  (bind _foundwidgets (`WidgetBlueprintLibrary.GetAllWidgetsOfClass` "/Game/BattleRoyale/WIdget/GameWidget/WG_MatchStartCountdown.WG_MatchStartCountdown_C" false))
  (for _array_element _foundwidgets
    (`/Game/BattleRoyale/WIdget/GameWidget/WG_MatchStartCountdown.Update_Widget` _array_element (`self.MatchStart_Countdown`))))

(fn `UserConstructionScript`
  (`parent.UserConstructionScript`))