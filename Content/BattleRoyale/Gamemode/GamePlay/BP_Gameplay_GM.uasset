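; BP_Gameplay_GM is the gameplay game mode for the Battle Royale mode, handling player join and leave notifications.
; PostLogin and OnLogout both call NotifyPlayerConnectionMessage on the game state, which owns the connection message logic.
; It contains no other active logic, as BeginPlay, Tick and the construction script are default stubs.
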(event `self.K2_PostLogin`
  (params (NewPlayer :type "PlayerController Object Reference"))
  (message `/Game/BattleRoyale/Gamemode/Interface/BPI_GameState.Notify_PlayerConnection` (`GameplayStatics.GetGameState`)))

(event `self.K2_OnLogout`
  (params (ExitingController :type "Controller Object Reference"))
  (message `/Game/BattleRoyale/Gamemode/Interface/BPI_GameState.Notify_PlayerConnection` (`GameplayStatics.GetGameState`)))

(fn `UserConstructionScript`
  (`parent.UserConstructionScript`))